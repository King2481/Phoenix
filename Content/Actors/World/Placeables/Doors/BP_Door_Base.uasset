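; Base Blueprint for placeable doors that characters can open, close or attack, with a white highlight on the mesh.
; Interaction toggles between Opening and Closing states when the lock component allows it, checking jammed, locked and whether the actor can unlock.
; A transition timeline plays or reverses to swing the mesh, then settles the state to Open or Closed.
; A refused interaction plays a short jiggle timeline instead.
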(event Custom|JiggleDoor
  ;[1 1 1] Jiggling the door
  (if (not (Audio|Components|Audio|IsPlaying (Variables|Default|GetJiggle%20Timeline)))
    (bind _dooralpha (Timeline|Jiggle%20Timeline PlayFromStart)
      (:Update
        (Transformation|SetRelativeRotation (Variables|Default|GetStaticMesh) (Math|Rotator|Lerp(Rotator) "0, 0, 0" "0.000000,2.500000,0.000000" _dooralpha) false false)))))

(event EventBlueprintonInteractedwith
  (params (InteractingActor :type Actor%20Object%20Reference))
  (if (CallFunction|CanOpenDoor InteractingActor)
    (Class|Door|TransitiontoState (select (Class|Door|IsOpenorOpening) "Closing" "Opening"))
    (else
      (CallFunction|JiggleDoor))))

(event EventBlueprintTransitiontoState
  (params (NewState :type EDoorState%20Enum :default "Closed"))
  ;[1 1 1] Opening the door
  (switch Utilities|FlowControl|Switch|SwitchonEDoorState NewState
    (:Closing
      (bind _dooralpha (Timeline|Transition%20Transition Reverse)
        (:Update
          (Transformation|SetRelativeRotation (Variables|Default|GetStaticMesh) (Math|Rotator|Lerp(Rotator) "0, 0, 0" "0.000000,90.000000,0.000000" _dooralpha) false false))
        (:Finished
          (Class|Door|TransitiontoState (select (Class|Door|IsOpenorOpening) "Open" "Closed")))))
    (:Opening
      (Timeline|Transition%20Transition Play))))

(fn ConstructionScript)

(fn GetMeshHighlightInfo
  (return (Utilities|Struct|MakeMeshHighlightInfo (Variables|Default|GetStaticMesh) "/Game/Materials/MI_Highlight_White.MI_Highlight_White")))

(fn GetPossibleInteractions
  (return (Utilities|Array|MakeArray (select (Class|Door|IsOpenorOpening) "/Game/Game/Interactions/Interaction_CloseDoor.Interaction_CloseDoor" "/Game/Game/Interactions/Interaction_OpenDoor.Interaction_OpenDoor") "/Game/Game/Interactions/Interaction_MainHandAttack.Interaction_MainHandAttack")))

(fn CanOpenDoor
  (params (OpeningActor :type Actor%20Object%20Reference))
  (bind _lockcomponent (Variables|Default|GetLockComponent))
  (if (Class|LockComponent|IsJammed _lockcomponent)
    (return false)
    (elif (Class|LockComponent|IsLocked _lockcomponent)
      (return (Class|LockComponent|CanUnlock (Variables|Default|GetLockComponent) OpeningActor))
      (else
        (return true)))))