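; Explosive barrel placeable that can be targeted and attacked, exploding when its health changes.
; Any health change event from the ability system triggers the Explosion component, then destroys the actor, with no check on the remaining health.
; It exposes its health, ability system, targeting and name as target info, offering main-hand attack as the only interaction and a red highlight on the cylinder mesh.
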(event ChangeHealthInfoDelegate(AbilitySystem)
  (params (NewModifyInfo :type Modify%20Health%20Info%20Structure%20%28by%20ref%29))
  (Class|ExplosionComponent|Explode (Variables|Default|GetExplosion) 0)
  (Actor|DestroyActor))

(event EventBeginPlay)

(event Collision|EventActorBeginOverlap
  (params (OtherActor :type Actor%20Object%20Reference)))

(event EventTick
  (params (DeltaSeconds :type Float%20%28single-precision%29)))

(fn ConstructionScript)

(fn GetPossibleInteractions
  (return (Utilities|Array|MakeArray "/Game/Game/Interactions/Interaction_MainHandAttack.Interaction_MainHandAttack")))

(fn GetMeshHighlightInfo
  (return (Utilities|Struct|MakeMeshHighlightInfo (Variables|Default|GetCylinder) "/Game/Materials/MI_Highlight_Red.MI_Highlight_Red")))

(fn GetTargetInfo
  (return (Utilities|Struct|MakeTargetableInfo (Variables|Default|GetHealth) (Variables|Default|GetAbilitySystem) (Variables|Default|GetTargetingComponent) (Class|NameComponent|GetEntityName (Variables|Default|GetNameComponent)) (CallFunction|GetPossibleInteractions))))