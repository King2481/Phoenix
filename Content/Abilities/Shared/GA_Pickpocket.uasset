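; Gameplay ability that walks the player to a target and opens the pickpocket screen.
; On activation it reads the first current target from the Phoenix ability system component and runs a simple move-to toward that target owner's location.
; A successful arrival displays the pickpocket screen asynchronously, with no EndAbility call on that path.
; Any other move result or a failed request ends the ability.
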(event Ability|EventActivateAbility
  (bind _asphoenix_ability_system_component (Utilities|Casting|CastToPhoenixAbilitySystemComponent (Ability|GetAbilitySystemComponentfromActorInfo)))
  (bind _result (|SimpleMoveto self (Game|GetPlayerController 0) 0 (Transformation|GetActorLocation (Components|GetOwner (Utilities|Array|Get(acopy) (Utilities|Struct|BreakTargetData (Class|PhoenixAbilitySystemComponent|GetCurrentTargetData _asphoenix_ability_system_component))))) 1e+02)
    (:OnMoveFinished
      (switch Utilities|FlowControl|Switch|SwitchonEPathFollowingResult _result
        (:Success
          (|DisplayPickpocketScreenAsync (Game|GetPlayerController 0)))
        (:Blocked
          (Ability|EndAbility :!label _label))
        (:OffPath
          (goto _label))
        (:Aborted
          (goto _label))
        (:Invalid
          (goto _label))))
    (:OnRequestFailed
      (Ability|EndAbility))))