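; Shared gameplay ability that acts as a dispatcher for the owner's main-hand attack.
; On activation it finds the owning actor's EquipmentManager and reads the weapon data in the main-hand slot.
; It then tries to activate that weapon's MainHandAttackAbility by class, with remote activation disallowed, and ends itself immediately, leaving the attack logic to the weapon-specific ability.
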(event Ability|EventActivateAbility
  (CallFunction|Attack)
  (Ability|EndAbility))

(event Ability|EventOnEndAbility
  (params (bWasCancelled :type Boolean)))

(fn Attack
  (bind _output_get (LocalVariables|SetEquipment (Actor|GetComponentbyClass (Ability|GetOwningActorfromActorInfo) "/Script/Phoenix.EquipmentManager")))
  (Utilities|IsValid _output_get
    (:Is%20Valid
      (bind _asitem_data_weapon (Utilities|Casting|CastToItemDataWeapon (Class|EquipmentManager|GetIteminSlot (LocalVariables|GetEquipment) "/Game/Actors/Items/EquipableSlots/EquipableSlot_MainHand.EquipableSlot_MainHand")))
      (Abilities|TryActivateAbilitybyClass (Ability|GetAbilitySystemComponentfromActorInfo) (Variables|/Script/Phoenix.ItemDataWeapon|GetMainHandAttackAbility _asitem_data_weapon) false))))