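; GA_Sneak is a gameplay ability that toggles sneaking on the owning Character.
; After committing, it checks whether the avatar is crouched: if so, it uncrouches and removes all GE_Sneak stacks, otherwise it crouches and applies GE_Sneak to itself.
; The ability ends immediately after each toggle or failed commit, leaving the effect to carry the sneak state, but a failed Character cast stops without ending it.
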(event Ability|EventActivateAbility
  (bind _returnvalue (Ability|CommitAbility))
  (if _returnvalue
    (bind _ascharacter (Utilities|Casting|CastToCharacter (Ability|GetOwningActorfromActorInfo)))
    (if (Variables|/Script/Engine.Character|GetbIsCrouched _ascharacter)
      (Character|UnCrouch _ascharacter)
      (GameplayEffects|RemoveActiveGameplayEffectbySourceEffect (Ability|GetAbilitySystemComponentfromActorInfo) "/Game/Abilities/Shared/GE_Sneak.GE_Sneak_C" 0 -1)
      (else
        (Character|Crouch _ascharacter)
        (GameplayEffects|ApplyGameplayEffectToSelf :self (Ability|GetAbilitySystemComponentfromActorInfo) :GameplayEffectClass "/Game/Abilities/Shared/GE_Sneak.GE_Sneak_C")))
    (Ability|EndAbility)
    (else
      (Ability|EndAbility))))

(event Ability|EventOnEndAbility
  (params (bWasCancelled :type Boolean)))