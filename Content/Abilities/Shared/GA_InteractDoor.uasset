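; Shared gameplay ability that lets the player open or close a targeted Door.
; It takes the door from the first target in the Phoenix ability system component's current target data and simple-moves the first player controller within range of it.
; A successful move toggles the door between Opening and Closing, then ends the ability.
; A failed move request ends the ability without changing the door.
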(event Ability|EventActivateAbility
  (bind _asphoenix_ability_system_component (Utilities|Casting|CastToPhoenixAbilitySystemComponent (Ability|GetAbilitySystemComponentfromActorInfo)))
  (bind _asdoor (Utilities|Casting|CastToDoor (Components|GetOwner (Utilities|Array|Get(acopy) (Utilities|Struct|BreakTargetData (Class|PhoenixAbilitySystemComponent|GetCurrentTargetData _asphoenix_ability_system_component))))))
  (Variables|Default|SetDoor _asdoor)
  (bind _result (|SimpleMoveto self (Game|GetPlayerController 0) 0 (Transformation|GetActorLocation (Components|GetOwner (Utilities|Array|Get(acopy) (Utilities|Struct|BreakTargetData (Class|PhoenixAbilitySystemComponent|GetCurrentTargetData _asphoenix_ability_system_component))))) 2.5e+02)
    (:OnMoveFinished
      (switch Utilities|FlowControl|Switch|SwitchonEPathFollowingResult _result
        (:Success
          (Class|Door|TransitiontoState (Variables|Default|GetDoor) (select (Class|Door|IsOpenorOpening (Variables|Default|GetDoor)) "Closing" "Opening")))))
    (:OnRequestFailed
      _))
  (Ability|EndAbility))