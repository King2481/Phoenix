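; Gameplay ability that lets the player pick the lock on a targeted door through a dice roll.
; It reads the door from the Phoenix ability system's current target data and moves the player within range using SimpleMoveTo.
; On arrival, a cancelable dice roll screen uses the lock component's difficulty class, and success unlocks the lock.
; Failed moves, closing or canceling the roll, and success all end the ability.
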(event Ability|EventActivateAbility
  (bind _asphoenix_ability_system_component (Utilities|Casting|CastToPhoenixAbilitySystemComponent (Ability|GetAbilitySystemComponentfromActorInfo)))
  (bind _asdoor (Utilities|Casting|CastToDoor (Components|GetOwner (Utilities|Array|Get(acopy) (Utilities|Struct|BreakTargetData (Class|PhoenixAbilitySystemComponent|GetCurrentTargetData _asphoenix_ability_system_component))))))
  (Variables|Default|SetDoor _asdoor)
  (bind _result (|SimpleMoveto self (Game|GetPlayerController 0) 0 (Transformation|GetActorLocation (Components|GetOwner (Utilities|Array|Get(acopy) (Utilities|Struct|BreakTargetData (Class|PhoenixAbilitySystemComponent|GetCurrentTargetData _asphoenix_ability_system_component))))) 1e+02)
    (:OnMoveFinished
      (switch Utilities|FlowControl|Switch|SwitchonEPathFollowingResult _result
        (:Success
          (|DisplayDiceRollScreenAsync (Game|GetPlayerController 0) (Utilities|Struct|MakeDiceRollScreenInfo (Variables|/Script/Phoenix.LockComponent|GetDifficultyClass (Variables|/Script/Phoenix.Door|GetLockComponent (Variables|Default|GetDoor))) true)
            (:OnSuccess
              (Class|LockComponent|SetLockState (Variables|/Script/Phoenix.Door|GetLockComponent (Variables|Default|GetDoor)) "Unlocked"))
            (:OnClose
              _)
            (:OnCanceled
              _)))
        (:Blocked
          _)
        (:OffPath
          _)
        (:Aborted
          _)
        (:Invalid
          _)))
    (:OnRequestFailed
      _))
  (Ability|EndAbility))