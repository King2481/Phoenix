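; Gameplay ability that walks the player to a loot target and opens a loot window there.
; It takes the first target in the Phoenix ability system component's current target data and runs a SimpleMoveTo task toward its owner using player controller 0.
; On success, the Phoenix player controller spawns the window with that owner's inventory items.
; The ability ends after success or a failed request; other move results leave it active.
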(event Ability|EventActivateAbility
  (bind _asphoenix_ability_system_component (Utilities|Casting|CastToPhoenixAbilitySystemComponent (Ability|GetAbilitySystemComponentfromActorInfo)))
  (bind _result (|SimpleMoveto self (Game|GetPlayerController 0) 0 (Transformation|GetActorLocation (Components|GetOwner (Utilities|Array|Get(acopy) (Utilities|Struct|BreakTargetData (Class|PhoenixAbilitySystemComponent|GetCurrentTargetData _asphoenix_ability_system_component))))) 1e+02)
    (:OnMoveFinished
      (switch Utilities|FlowControl|Switch|SwitchonEPathFollowingResult _result
        (:Success
          (bind _asphoenix_player_controller (Utilities|Casting|CastToPhoenixPlayerController (Game|GetPlayerController 0))
            (:then
              (Class|PhoenixPlayerController|SpawnLootWindowatLocation _asphoenix_player_controller (Transformation|GetActorLocation (Components|GetOwner (Utilities|Array|Get(acopy) (Utilities|Struct|BreakTargetData (Class|PhoenixAbilitySystemComponent|GetCurrentTargetData _asphoenix_ability_system_component))))) (Class|InventoryComponent|GetInventoryItems (Actor|GetComponentbyClass (Components|GetOwner (Utilities|Array|Get(acopy) (Utilities|Struct|BreakTargetData (Class|PhoenixAbilitySystemComponent|GetCurrentTargetData _asphoenix_ability_system_component)))) "/Script/Phoenix.InventoryComponent"))))
            (:CastFailed
              _)))))
    (:OnRequestFailed
      _))
  (Ability|EndAbility))