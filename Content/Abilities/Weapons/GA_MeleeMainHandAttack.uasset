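; GA_MeleeMainHandAttack is a gameplay ability for a main-hand melee attack, currently an early stub.
; On activation it takes the first target from the Phoenix ability system component's current target data and runs a SimpleMoveTo task on player 0's controller toward that target's owner.
; A successful move only prints a debug message, with no attack logic yet, while a failed request ends the ability.
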(event Ability|EventActivateAbility
  (bind _asphoenix_ability_system_component (Utilities|Casting|CastToPhoenixAbilitySystemComponent (Ability|GetAbilitySystemComponentfromActorInfo)))
  (bind _result (|SimpleMoveto self (Game|GetPlayerController 0) 0 (Transformation|GetActorLocation (Components|GetOwner (Utilities|Array|Get(acopy) (Utilities|Struct|BreakTargetData (Class|PhoenixAbilitySystemComponent|GetCurrentTargetData _asphoenix_ability_system_component))))) 1e+02)
    (:then
      (switch Utilities|FlowControl|Switch|SwitchonEPathFollowingResult _result
        (:Success
          (Development|PrintString "Hello"))))
    (:OnRequestFailed
      (Ability|EndAbility))))

(event Ability|EventOnEndAbility
  (params (bWasCancelled :type Boolean)))