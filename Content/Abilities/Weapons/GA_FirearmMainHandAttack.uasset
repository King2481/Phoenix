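; Gameplay ability for a main-hand firearm attack on the first target in the Phoenix ability system's current target data.
; A FaceTarget task turns toward the target, then the main-hand item's spawned prop queues and fires bullets through its BulletFiringComponent.
; Bullet count comes from the first fire mode, and loaded ammo lowers the crit die.
; Hit rolls are off and bullet data is hardcoded to 12-gauge buckshot.
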(event Ability|EventActivateAbility
  (bind _returnvalue (Ability|GetAbilitySystemComponentfromActorInfo))
  (bind _asphoenix_ability_system_component (Utilities|Casting|CastToPhoenixAbilitySystemComponent _returnvalue))
  (|FaceTarget self (Components|GetOwner (Utilities|Array|Get(acopy) (Utilities|Struct|BreakTargetData (Class|PhoenixAbilitySystemComponent|GetCurrentTargetData (.AsPhoenix%20Ability%20System%20Component (Utilities|Casting|CastToPhoenixAbilitySystemComponent (Ability|GetAbilitySystemComponentfromActorInfo))))))) 7.5
    (:OnRequestFinished
      (bind _output_get (Variables|Default|SetEquipment (Actor|GetComponentbyClass (Ability|GetOwningActorfromActorInfo) "/Script/Phoenix.EquipmentManager")))
      (Utilities|IsValid _output_get
        (:Is%20Valid
          (bind _asitem_data_firearm (Utilities|Casting|CastToItemDataFirearm (Class|EquipmentManager|GetIteminSlot (Variables|Default|GetEquipment) "/Game/Actors/Items/EquipableSlots/EquipableSlot_MainHand.EquipableSlot_MainHand")))
          (Class|BulletFiringComponent|QueueandFireBullets (Actor|GetComponentbyClass (Variables|/Script/Phoenix.ItemDataHandEquipable|GetSpawnedProp _asitem_data_firearm) "/Script/Phoenix.BulletFiringComponent") (Utilities|Struct|MakeFireBulletQueueInfo (.bulletstofire (Utilities|Array|Get(acopy) (Variables|/Script/Phoenix.ItemDataFirearm|GetAvailableFireModes _asitem_data_firearm))) (- (Variables|/Script/Phoenix.ItemDataWeapon|GetCritDie _asitem_data_firearm) (Class|AmmoComponent|GetCritDieBonusfromLoadedAmmo (Actor|GetComponentbyClass (Variables|/Script/Phoenix.ItemDataHandEquipable|GetSpawnedProp _asitem_data_firearm) "/Script/Phoenix.AmmoComponent"))) false "/Game/Actors/Items/Weapons/Ammo/BulletFiringData/BFD_12GBuckshot.BFD_12GBuckshot" _asphoenix_ability_system_component (Utilities|Array|Get(acopy) (Utilities|Struct|BreakTargetData (Class|PhoenixAbilitySystemComponent|GetCurrentTargetData _asphoenix_ability_system_component)))))
          (Ability|EndAbility))))))

(event Ability|EventOnEndAbility
  (params (bWasCancelled :type Boolean)))